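; Torch actor with a point light and particle fire whose color reflects its goal role and the game's clear state.
; The construction script tints both the light and the particle FireColor parameter blue when IsGoal is set.
; At BeginPlay, both turn red if the level is "End" and the AwardGameInstance IsClear flag is false, overriding any goal tint.
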(event `self.ReceiveBeginPlay`
  (bind _returnvalue (`GameplayStatics.GetCurrentLevelName` true))
  (if (and (`KismetStringLibrary.EqualEqual_StrStr` _returnvalue "End") (not (`/Game/BP/AwardGameInstance.IsClear` (cast `/Game/BP/AwardGameInstance` (`GameplayStatics.GetGameInstance`) :!pure true))))
    (`LightComponent.SetLightColor` (`self.PointLight`) (struct :`R` 1.0 :`A` 1.0) true)
    (`ParticleSystemComponent.SetColorParameter` (`self.ParticleSystem`) "FireColor" (struct :`R` 1.0 :`A` 1.0))))

(fn `UserConstructionScript`
  (if (`self.IsGoal`)
    (`LightComponent.SetLightColor` (`self.PointLight`) (struct :`B` 1.0 :`A` 1.0) true)
    (`ParticleSystemComponent.SetColorParameter` (`self.ParticleSystem`) "FireColor" (struct :`G` 0.25 :`B` 10.0 :`A` 1.0))))