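; Stair goal trigger that ends the current stage when a BP_Award actor overlaps its GoalBox.
; It plays a stair sound for the GameInstance's LoadingTime, then stops it and shows the GameMode's loading widget for another equal delay.
; On the last stage it sets IsClear on the GameInstance and opens the End level.
; Otherwise it hides the widget and calls NextStage on BP_AwardGameMode.
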(event `self.GoalBox.OnComponentBeginOverlap`
  (params (OverlappedComponent :type "PrimitiveComponent Object Reference") (OtherActor :type "Actor Object Reference") (OtherComp :type "PrimitiveComponent Object Reference") (OtherBodyIndex :type Integer) (bFromSweep :type Boolean) (SweepResult :type "HitResult Structure (by ref)"))
  (bind _asbp_award_game_mode (cast `/Game/BP/BP_AwardGameMode` (`GameplayStatics.GetGameMode`) :!pure true))
  (bind _asaward_game_instance (cast `/Game/BP/AwardGameInstance` (`GameplayStatics.GetGameInstance`) :!pure true))
  (bind _loadingwidget (`/Game/BP/BP_AwardGameMode.LoadingWidget` _asbp_award_game_mode))
  (bind _loadingtime (`/Game/BP/AwardGameInstance.LoadingTime` _asaward_game_instance))
  (cast `/Game/BP/BP_Award` OtherActor)
  (bind _returnvalue (`GameplayStatics.SpawnSound2D` "/Game/Audio/stair.stair"))
  (`KismetSystemLibrary.Delay` _loadingtime)
  (`ActorComponent.SetActive` _returnvalue false false)
  (`Widget.SetVisibility` _loadingwidget "Visible")
  (`KismetSystemLibrary.Delay` _loadingtime)
  (if (`self.LastStage`)
    (set `/Game/BP/AwardGameInstance.IsClear` true _asaward_game_instance)
    (`GameplayStatics.OpenLevel` "End")
    (else
      (`Widget.SetVisibility` _loadingwidget "Hidden")
      (`/Game/BP/BP_AwardGameMode.NextStage` _asbp_award_game_mode))))

(fn `UserConstructionScript`)